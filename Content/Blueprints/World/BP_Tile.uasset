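; BP_Tile is a world tile that can populate itself with an enemy when play begins.
; On BeginPlay it makes a one-in-four random roll, then traces a short line upward for WorldDynamic objects to check that the space is free.
; If nothing is hit, it spawns a BP_Enemy above itself, adjusting for collisions, and registers it through SetCharacterOnTile.
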(event EventBeginPlay
  (bind _returnvalue (Transformation|GetActorLocation))
  (if (<= (Math|Random|RandomIntegerinRange 1 100) 25)
    (bind _outhit (Collision|LineTraceForObjects _returnvalue (+ _returnvalue "0, 0,100.000000") (Utilities|Array|MakeArray "ObjectTypeQuery2") false (Utilities|Array|MakeArray self) "None"))
    (Utilities|IsValid (.HitActor (Collision|BreakHitResult _outhit))
      (:Is%20Not%20Valid
        (bind _returnvalue_2 (Game|SpawnActorfromClass "/Game/Blueprints/Characters/BP_Enemy.BP_Enemy_C" (Math|Transform|MakeTransform (+ (Transformation|GetActorLocation) "0, 0,100.000000") "0, 0, 0" "1,1,1") "AdjustIfPossibleButDontSpawnIfColliding" 0 0))
        (Class|BaseTile|SetCharacteronTile _returnvalue_2)))))

(event Collision|EventActorBeginOverlap
  (params (OtherActor :type Actor%20Object%20Reference)))

(event EventTick
  (params (DeltaSeconds :type Float%20%28single-precision%29)))

(fn ConstructionScript)