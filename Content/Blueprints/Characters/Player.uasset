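; Player character Blueprint that drives grid-based, step-by-step movement from keyboard input.
; W, A, S and D call Move on a GridMovement component for forward, left, backward and right steps.
; Q and E call Turn on the same component to rotate left or right.
; All movement logic lives in that component; the Blueprint only forwards raw key presses.
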(event EventBeginPlay)

(event Collision|EventActorBeginOverlap
  (params (OtherActor :type Actor%20Object%20Reference)))

(event EventTick
  (params (DeltaSeconds :type Float%20%28single-precision%29)))

(event Input|KeyboardEvents|W
  (params (Key :type Key%20Structure :default "None"))
  (:Pressed
    (Class|GridMovement|Move (Variables|Default|GetGridMovement) "Forward")))

(event Input|KeyboardEvents|A
  (params (Key :type Key%20Structure :default "None"))
  (:Pressed
    (Class|GridMovement|Move (Variables|Default|GetGridMovement) "Left")))

(event Input|KeyboardEvents|S
  (params (Key :type Key%20Structure :default "None"))
  (:Pressed
    (Class|GridMovement|Move (Variables|Default|GetGridMovement) "Backward")))

(event Input|KeyboardEvents|D
  (params (Key :type Key%20Structure :default "None"))
  (:Pressed
    (Class|GridMovement|Move (Variables|Default|GetGridMovement) "Right")))

(event Input|KeyboardEvents|Q
  (params (Key :type Key%20Structure :default "None"))
  (:Pressed
    (Class|GridMovement|Turn (Variables|Default|GetGridMovement) "Left")))

(event Input|KeyboardEvents|E
  (params (Key :type Key%20Structure :default "None"))
  (:Pressed
    (Class|GridMovement|Turn (Variables|Default|GetGridMovement) "Right")))

(fn ConstructionScript)